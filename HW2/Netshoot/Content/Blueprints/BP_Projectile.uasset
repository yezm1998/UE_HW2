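; Projectile that scores a point for its instigator when it overlaps a BP_MyProjectile whose root component is tagged "Sphere".
; Every overlap plays an attenuated sound with random pitch; a qualifying hit adds a second, quieter sound.
; On that hit, only the authority increments the instigator's MyPlayerState score and destroys both actors.
; Any other overlap destroys just this projectile, without an authority check.
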(event Collision|EventActorBeginOverlap
  (params (OtherActor :type Actor%20Object%20Reference))
  ;[0 1 0] Sound
  (Audio|PlaySoundatLocation "/Game/Sounds/SoundCue_Attentuated.SoundCue_Attentuated" "0, 0, 0" "0, 0, 0" (Variables|Default|GetVolumeMultiplier) (Math|Random|RandomFloatinRange 0.8 1.2) 0.0 0 0 0)
  (Utilities|Casting|CastToBP_MyProjectile OtherActor
    (:then
      (if (Components|ComponentHasTag (Variables|/Script/Engine.Actor|GetRootComponent OtherActor) "Sphere")
        ;[0 1 0] Sound
        (Audio|PlaySoundatLocation "/Game/Sounds/Randomize_01.Randomize_01" "0, 0, 0" "0, 0, 0" (* (Variables|Default|GetVolumeMultiplier) 0.25) 1.0 0.0 0 0 0)
        (Networking|SwitchHasAuthority
          (:Authority
            (bind _asmy_player_state (Utilities|Casting|CastToMyPlayerState (Variables|/Script/Engine.Controller|GetPlayerState (Game|GetInstigatorController))))
            (Default|IncrementScore _asmy_player_state)
            (Actor|DestroyActor OtherActor)))))
    (:CastFailed
      _))
  ;[1 1 1] Hit Hat
  (Actor|DestroyActor self))

(fn ConstructionScript)